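; Inventory manager actor that tracks champions and items in on-board and off-board lists.
; On BeginPlay it spawns a champion at the next bench slot, chosen by the off-board champion count and placed at a fixed height, then adds it to that list.
; DropItem always spawns the given item class at its transform, adds the new actor to the on-board items and removes that same actor from the off-board items.
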(event EventBeginPlay
  (bind _worldposition (CallFunction|ChampionLocationonSpawn))
  (bind _returnvalue (Game|SpawnActorfromClass "/Game/Wander/Blueprints/Characters/Champion_BP.Champion_BP_C" (Math|Transform|MakeTransform _worldposition "0, 0, 0" "1,1,1") "Undefined" 0 0))
  (Utilities|Set|Add (Variables|Default|GetOffBoardChampions) _returnvalue))

(event Collision|EventActorBeginOverlap
  (params (OtherActor :type Actor%20Object%20Reference)))

(event EventTick
  (params (DeltaSeconds :type Float%20%28single-precision%29)))

(fn ConstructionScript)

(fn DropItem
  (params (DropStruct :type Drop%20Struct%20Structure))
  (bind (_itemclass _proxyclass _transform) (Utilities|Struct|BreakDrop_Struct DropStruct))
  (bind _returnvalue (Game|SpawnActorfromClass _itemclass _transform "AlwaysSpawn" 0 0 0))
  (Utilities|Set|Add (Variables|Default|GetOnBoardItems) _returnvalue)
  (Utilities|Set|Remove (Variables|Default|GetOffBoardItems) _returnvalue))

(fn ChampionLocationonSpawn
  (bind _slotworldposition (CallFunction|GetBenchSlotWorldPosition (Utilities|Set|Length (Variables|Default|GetOffBoardChampions))))
  (return (Math|Vector|MakeVector (.x _slotworldposition) (.y _slotworldposition) 1.5e+02)))