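; Champion character that the player picks up and places on bench or board squares, with hover highlight and randomized body color.
; Clicking it removes it from its square and opens a Tick gate that makes it follow the cursor.
; DropChampion traces down to find the square center, then checks GameState for occupancy and capacity.
; Dropping onto an occupied square picks up the displaced champion, keeping carry mode active.
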(event Custom|OpenTickGate
  (bind _cursorworldposition (Variables|Default|GetCursorWorldPosition))
  (Utilities|FlowControl|Gate true) ; enters at Open
)

(event Custom|CloseTickGate
  (bind _cursorworldposition (Variables|Default|GetCursorWorldPosition))
  (Utilities|FlowControl|Gate true) ; enters at Close
)

(event Custom|OnPickedUpModeActivated)

(event Custom|OnPickedUpModeDeactivated_Event
  (Variables|/Game/Wander/Blueprints/CameraPawnController.CameraPawnController_C|SetDropCharacterModeActive (Variables|Default|GetControllerRef) false))

(event EventBeginPlay
  (bind _returnvalue (Game|GetPlayerController 0))
  (|CallParentFunction)
  (Variables|/Script/Engine.PlayerController|SetbShowMouseCursor _returnvalue true)
  (Variables|/Script/Engine.PlayerController|SetbEnableMouseOverEvents _returnvalue true)
  (Utilities|Struct|SetmembersinCharacterProfile_Struct (Variables|Default|GetMyProfile) "NewEnumerator2")
  (EventDispatchers|BindEventtoPickedUpModeActivated (delegate Custom|OnPickedUpModeActivated))
  (EventDispatchers|BindEventtoOnPickedUpModeDeactivated (delegate Custom|OnPickedUpModeDeactivated_Event)))

(event Collision|EventActorBeginOverlap
  (params (OtherActor :type Actor%20Object%20Reference)))

(event EventTick
  (params (DeltaSeconds :type Float%20%28single-precision%29))
  (bind _cursorworldposition (Variables|Default|GetCursorWorldPosition))
  (|CallParentFunction 0.0)
  (Utilities|FlowControl|Gate true
    (:Exit
      (Utilities|GetCursorWorldPosition
        (:Out
          (Transformation|SetActorLocation self (Math|Vector|MakeVector (.x _cursorworldposition) (.y _cursorworldposition) 2e+02) false false))))))

(event MouseInput|EventActorOnClicked
  (params (ButtonPressed :type Key%20Structure))
  (if (not (Variables|Default|GetisPickedUp))
    (if (not (Variables|/Game/Wander/Blueprints/CameraPawnController.CameraPawnController_C|GetDropCharacterModeActive (Variables|Default|GetControllerRef)))
      (CallFunction|PickUpChampion))))

(event MouseInput|EventActorBeginCursorOver
  (Rendering|SetRenderCustomDepth (Variables|/Script/Engine.Character|GetMesh self) true))

(event MouseInput|EventActorEndCursorOver
  (Rendering|SetRenderCustomDepth (Variables|/Script/Engine.Character|GetMesh self) false))

(fn ConstructionScript
  (|CallParentFunction)
  (bind _returnvalue (Rendering|Material|CreateDynamicMaterialInstance (Variables|Character|GetMesh) 0 "/Game/AnimStarterPack/UE4_Mannequin/Materials/M_UE4Man_Body.M_UE4Man_Body" "None" :!class /Script/Engine.PrimitiveComponent))
  (bind _output_get (LocalVariables|SetColorValue (Utilities|Struct|MakeLinearColor (Math|Random|RandomFloatinRange 0.0 1.0) (Math|Random|RandomFloatinRange 0.0 1.0) (Math|Random|RandomFloatinRange 0.0 1.0) 1.0)))
  (Rendering|Material|SetVectorParameterValue _returnvalue "BodyColor" _output_get :!class /Script/Engine.MaterialInstanceDynamic))

(fn GetSquareCenterPosition
  (bind _self self)
  (bind _returnvalue (Transformation|GetActorLocation _self))
  (bind (_outhit _returnvalue_2) (Collision|LineTraceForObjects _returnvalue (- _returnvalue "0, 0,1000.000000") (Utilities|Array|MakeArray "ObjectTypeQuery7") false 0 "Persistent"))
  (if _returnvalue_2
    (Utilities|Casting|CastToBenchSquare (.hitactor _outhit)
      (:then
        (LocalVariables|SetisBenchPos true))
      (:CastFailed
        (LocalVariables|SetisBenchPos false)))
    (return true (Transformation|GetActorLocation (.hitactor _outhit)) (LocalVariables|GetisBenchPos))
    (else
      (return false "0, 0, 0" false))))

(fn GetMyGameState
  (bind _asmy_game_state (Utilities|Casting|CastToMyGameState (Game|GetGameState)))
  (return _asmy_game_state))

(fn PickUpChampion
  (bind _controllerref (Variables|Default|GetControllerRef))
  (CallFunction|OpenTickGate)
  (Variables|Default|SetisPickedUp true)
  (Variables|/Game/Wander/Blueprints/CameraPawnController.CameraPawnController_C|SetDropCharacterModeActive _controllerref true)
  (Variables|/Game/Wander/Blueprints/CameraPawnController.CameraPawnController_C|SetPickedUpChampionRef _controllerref self)
  (if (Variables|Default|GetisInPlay)
    (CallFunction|RemoveCharacterfromBoard)
    (else
      (CallFunction|RemoveCharacterfromBench))))

(fn DropChampion
  (bind (_isvaliddropposition _returnvalue _isbenchposition) (CallFunction|GetSquareCenterPosition))
  (Variables|Default|SetNewSquareX (.x _returnvalue))
  (Variables|Default|SetNewSquareY (.y _returnvalue))
  (if _isvaliddropposition
    (if _isbenchposition
      (|DropOntoBench (.x _returnvalue) (.y _returnvalue))
      (else
        (|DropOntoBoard (.x _returnvalue) (.y _returnvalue))))))