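; Base unit for what appears to be an auto-battler, holding combat state copied from its profile at construction.
; Board and bench functions update its position and in-play flag and sync with MyGameState.
; The controller's start-attacking event starts a looping attack-speed timer that fires homing missiles at the aggroed enemy.
; Tick checks health, disabling collision and destroying the dead unit after a delay; random minion coloring is left unwired.
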(event Custom|OnStartAttacking
  (Utilities|Time|SetTimerbyFunctionName self "FireAttack" (/ 1.0 (.currentattackspeed (Variables|Default|GetMyState))) true))

(event EventBeginPlay
  (Development|PrintString "char event begin play!")
  (EventDispatchers|BindEventtoStartAttacking (Variables|Default|GetControllerRef) (delegate Custom|OnStartAttacking)))

(event Collision|EventActorBeginOverlap
  (params (OtherActor :type Actor%20Object%20Reference)))

(event EventTick
  (params (DeltaSeconds :type Float%20%28single-precision%29))
  (|CheckHealth
    (:false
      (if (Variables|/Game/Wander/Blueprints/CameraPawnController.CameraPawnController_C|GetBattleModeActive (Variables|Default|GetControllerRef))
        (if (Variables|Default|GetisAttacking)
          _)))))

(fn ConstructionScript
  (CallFunction|InitializeState))

(fn RandomMinionFeatures
  (bind _returnvalue (Rendering|Material|CreateDynamicMaterialInstance (Variables|Character|GetMesh) 0 "/Game/Mannequin/Character/Materials/M_UE4Man_Body_Inst.M_UE4Man_Body_Inst" "None" :!class /Script/Engine.PrimitiveComponent))
  (LocalVariables|SetMaterialInstance _returnvalue)
  (LocalVariables|SetRandomType (Utilities|Enum|LiteralenumMinionType_ENUM (Utilities|Enum|ByteToEnumMinionType_ENUM (Math|Conversions|ToByte(Integer) (Math|Random|RandomIntegerinRange 0 2))))))

(fn InitializeState
  (bind _myprofile (Variables|Default|GetMyProfile))
  (Variables|Default|SetMyState (Utilities|Struct|MakeCharacterState_Struct (.maxhealthbase _myprofile) (.attackspeedbase _myprofile) (.attackdamagebase _myprofile) (.attackrangebase _myprofile) (Utilities|Set|MakeSet 0) 0 0)))

(fn GetCharacterState
  (return (Variables|Default|GetMyState)))

(fn SetCharacterAggro
  (params (ChampionToAggro :type Auto%20Character%20BP%20Object%20Reference))
  (Utilities|Struct|SetmembersinCharacterState_Struct (Variables|Default|GetMyState) ChampionToAggro))

(fn GetCharacterAggroed
  (return (.enemyaggroed (Variables|Default|GetMyState))))

(fn GetCharacterAttackRange
  (return (.currentattackrange (Variables|Default|GetMyState))))

(fn GetBoardPosition
  (return (.position (Variables|Default|GetMyState))))

(fn GetCharacterType
  (return (.charactertype (Variables|Default|GetMyProfile))))

(fn MoveCharacterBoardPosition
  (params (NewPosition :type Integer))
  (LocalVariables|SetOldPosition (.position (Variables|Default|GetMyState)))
  (Utilities|Struct|SetmembersinCharacterState_Struct (Variables|Default|GetMyState) NewPosition)
  (bind _asmy_game_state (Utilities|Casting|CastToMyGameState (Game|GetGameState)))
  (Default|MoveCharacterBoardPosition _asmy_game_state self NewPosition (LocalVariables|GetOldPosition) false)
  (Variables|Default|SetisInPlay true))

(fn IsCharinPlay
  (return (Variables|Default|GetisInPlay)))

(fn RemoveCharacterfromBoard
  (bind _asmy_game_state (Utilities|Casting|CastToMyGameState (Game|GetGameState)))
  (Default|RemoveCharacterfromBoard _asmy_game_state (.position (Variables|Default|GetMyState)))
  (Variables|Default|SetisInPlay false))

(fn PickUpCharacter)

(fn RemoveCharacterfromBench
  (bind _asmy_game_state (Utilities|Casting|CastToMyGameState (Game|GetGameState)))
  (Default|RemoveCharacterfromBench _asmy_game_state (.position (Variables|Default|GetMyState))))

(fn AddCharactertoBoard
  (params (Position :type Integer))
  (bind _asmy_game_state (Utilities|Casting|CastToMyGameState (Game|GetGameState)))
  (Default|AddCharactertoBoard _asmy_game_state self Position)
  (Utilities|Struct|SetmembersinCharacterState_Struct (Variables|Default|GetMyState) Position)
  (Variables|Default|SetisInPlay true))

(fn AddCharactertoBench
  (params (Position :type Integer))
  (bind _asmy_game_state (Utilities|Casting|CastToMyGameState (Game|GetGameState)))
  (Default|AddCharactertoBench _asmy_game_state self Position)
  (Utilities|Struct|SetmembersinCharacterState_Struct (Variables|Default|GetMyState) Position)
  (Variables|Default|SetisInPlay false))

(fn AddNewCharactertoBench
  (bind _asmy_game_state (Utilities|Casting|CastToMyGameState (Game|GetGameState)))
  (bind _newchampposition (Default|AddNewChamptoBench _asmy_game_state self))
  (Utilities|Struct|SetmembersinCharacterState_Struct (Variables|Default|GetMyState) _newchampposition)
  (Variables|Default|SetisInPlay false)
  (return _newchampposition))

(fn FireAttack
  (bind _returnvalue (Transformation|GetActorLocation))
  (bind _returnvalue_2 (Transformation|GetActorForwardVector))
  (bind _mystate (Variables|Default|GetMyState))
  (bind _returnvalue_3 (* _returnvalue_2 110))
  (bind _returnvalue_4 (+ _returnvalue _returnvalue_3))
  (bind _output_get (LocalVariables|SetmyEnemyAggroed (.enemyaggroed _mystate)))
  (if (!= (.enemyaggroed _mystate) 0)
    (Transformation|SetRelativeRotation (Variables|Character|GetMesh) (Math|Rotator|FindLookatRotation (Transformation|GetActorLocation self) (Transformation|GetActorLocation _output_get)) false false)
    (bind _returnvalue_5 (Game|SpawnActorfromClass "/Game/Wander/Blueprints/Projectiles/MissileBP.MissileBP_C" (Math|Transform|MakeTransform (Math|Vector|MakeVector (.x _returnvalue_4) (.y _returnvalue_4) (+ (.z _returnvalue_4) 38.0)) (Transformation|GetActorRotation) "0.200000,0.200000,0.200000") "Undefined" 0 0))
    (Variables|/Script/Engine.ProjectileMovementComponent|SetHomingTargetComponent (Variables|/Game/Wander/Blueprints/Projectiles/MissileBP.MissileBP_C|GetProjectileMovement _returnvalue_5) (Variables|/Script/Engine.Character|GetMesh (LocalVariables|GetmyEnemyAggroed)))
    (Variables|/Script/Engine.ProjectileMovementComponent|SetbIsHomingProjectile (Variables|/Game/Wander/Blueprints/Projectiles/MissileBP.MissileBP_C|GetProjectileMovement _returnvalue_5) true)
    (Variables|/Script/Engine.ProjectileMovementComponent|SetHomingAccelerationMagnitude (Variables|/Game/Wander/Blueprints/Projectiles/MissileBP.MissileBP_C|GetProjectileMovement _returnvalue_5) 2.5e+04)))