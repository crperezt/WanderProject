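; Ghost preview actor for drop-item mode, showing the selected item's mesh and following the cursor at a fixed height.
; DropItem briefly spawns the item to read its mesh and inventory proxy, then resets and activates the ghost, toggling the controller's drop-mode flag and a gated Tick.
; GetDropStruct packages the drop data, using a downward trace to center it on a grid square or flag it off-board.
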(event Custom|OnSpawn
  (params (DisplayMesh :type Static%20Mesh%20Object%20Reference) (ItemClass :type Item%20Master%20BP%20Class%20Reference) (InventoryProxy :type Inventory%20Proxy%20Class%20Reference))
  (if (not (Variables|Default|GetisActive))
    (Variables|Default|SetItemClass ItemClass)
    (Variables|Default|SetInventoryProxy InventoryProxy)
    (Variables|Default|SetDisplayMesh DisplayMesh)
    (Variables|Default|SetisActive true)
    (Variables|/Game/Wander/Blueprints/CameraPawnController.CameraPawnController_C|SetDropItemModeActive (Variables|Default|GetControllerRef) true)
    (Components|StaticMesh|SetStaticMesh (Variables|Default|GetGhostItem_Mesh) (Variables|Default|GetDisplayMesh))
    (CallFunction|OpenTickGate)))

(event Custom|KillGhost
  (Variables|Default|SetItemClass 0)
  (Variables|Default|SetInventoryProxy 0)
  (CallFunction|CloseTickGate)
  (Variables|Default|SetDisplayMesh 0)
  (Variables|Default|SetisActive false)
  (Variables|/Game/Wander/Blueprints/CameraPawnController.CameraPawnController_C|SetDropItemModeActive (Variables|Default|GetControllerRef) false)
  (Components|StaticMesh|SetStaticMesh (Variables|Default|GetGhostItem_Mesh) (Variables|Default|GetDisplayMesh)))

(event Custom|OpenTickGate
  (bind _cursorworldposition (Variables|Default|GetCursorWorldPosition))
  (Utilities|FlowControl|Gate true) ; enters at Open
)

(event Custom|CloseTickGate
  (bind _cursorworldposition (Variables|Default|GetCursorWorldPosition))
  (Utilities|FlowControl|Gate true) ; enters at Close
)

(event EventBeginPlay)

(event EventDropItem
  (params (Item :type Item%20Master%20BP%20Class%20Reference))
  (bind _returnvalue (Game|SpawnActorfromClass Item (Math|Transform|MakeTransform "0, 0, 0") "Undefined" 0 (Variables|Default|GetControllerRef) 0))
  (Utilities|FlowControl|Sequence
    (:then_0
      (bind _asitem_master_bp (Utilities|Casting|CastToItemMaster_BPClass Item))
      (CallFunction|KillGhost)
      (CallFunction|OnSpawn (Variables|/Game/Wander/Blueprints/Items/ItemMaster_BP.ItemMaster_BP_C|GetDisplayMesh _returnvalue) _asitem_master_bp (Variables|/Game/Wander/Blueprints/Items/ItemMaster_BP.ItemMaster_BP_C|GetInventoryProxy _returnvalue)))
    (:then_1
      (Actor|DestroyActor _returnvalue))))

(event Collision|EventActorBeginOverlap
  (params (OtherActor :type Actor%20Object%20Reference)))

(event EventTick
  (params (DeltaSeconds :type Float%20%28single-precision%29))
  (bind _cursorworldposition (Variables|Default|GetCursorWorldPosition))
  (Utilities|FlowControl|Gate true
    (:Exit
      (Transformation|SetActorLocation self (Math|Vector|MakeVector (.x _cursorworldposition) (.y _cursorworldposition) 1e+02) false false))))

(fn ConstructionScript)

(fn SetGridSnapVector
  (bind _cursorworldposition (Variables|Default|GetCursorWorldPosition))
  (bind _gridsize (Variables|Default|GetGridSize))
  (return (Math|Vector|MakeVector (CallFunction|GridSnap (.x _cursorworldposition) _gridsize) (CallFunction|GridSnap (.y _cursorworldposition) _gridsize) (CallFunction|GridSnap (.z _cursorworldposition) _gridsize))))

(fn SetCursorPosition
  (params (CursorLocation :type Vector))
  (Variables|Default|SetCursorWorldPosition CursorLocation)
  (return))

(fn GetDropStruct
  (bind (_isoffboard _droplocation) (CallFunction|GetDropLocation))
  (return (Utilities|Struct|MakeDrop_Struct (Variables|Default|GetItemClass) (Variables|Default|GetInventoryProxy) (Math|Transform|MakeTransform (Math|Vector|MakeVector (.x _droplocation) (.y _droplocation) 8e+01) (Transformation|GetActorRotation)) (Variables|Default|GetDisplayMesh) 1.0) _isoffboard))

(fn HighlightSquares
  (params (location :type Vector))
  (bind (_outhit _returnvalue) (Collision|LineTraceForObjects location (- location "0, 0,300.000000") (Utilities|Array|MakeArray "ObjectTypeQuery7") false 0 "None"))
  (if _returnvalue
    _))

(fn GetDropLocation
  (bind (_outhit _returnvalue) (Collision|LineTraceForObjects (Transformation|GetActorLocation self) (- (Variables|Default|GetCursorWorldPosition) "0, 0,300.000000") (Utilities|Array|MakeArray "ObjectTypeQuery7") false 0 "None"))
  (if _returnvalue
    (return false (Transformation|GetActorLocation (.hitactor _outhit)))
    (else
      (return true "0, 0, 0"))))